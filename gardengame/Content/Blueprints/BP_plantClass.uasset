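; BP_plantClass is a plant actor that visually reflects its GrownPercent, which is not modified in this Blueprint.
; The construction script applies a dynamic instance of the Circuit material to the mesh, and BeginPlay stores its BP_soil owner.
; Each Tick scales the actor with growth while it is not at 100 percent, then switches on material emission at full growth instead of rescaling.
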(event EventBeginPlay
  (bind _asbp_soil (Utilities|Casting|CastToBP_soil (Components|GetOwner)))
  (Variables|Default|Setsoil _asbp_soil))

(event EventTick
  (params (DeltaSeconds :type Float%20%28single-precision%29))
  (bind _grownpercent (Variables|Default|GetgrownPercent))
  (if (== _grownpercent 100)
    (Rendering|Material|SetScalarParameterValue (Variables|Default|GetdynamicMaterial) "emission" 0.5 :!class /Script/Engine.MaterialInstanceDynamic)
    (else
      (Transformation|SetActorScale3D (Math|Conversions|ToVector(Float) (Math|Float|Lerp 0.2 1.0 (/ (Math|Conversions|ToFloat(Integer) _grownpercent) 1e+02))))
      (Rendering|Material|SetScalarParameterValue (Variables|Default|GetdynamicMaterial) "emission" 0.0 :!class /Script/Engine.MaterialInstanceDynamic))))

(fn ConstructionScript
  (bind _returnvalue (Rendering|Material|CreateDynamicMaterialInstance "/Game/Shaders/circuit.circuit" "None" :!class /Script/Engine.KismetMaterialLibrary))
  (bind _output_get (Variables|Default|SetdynamicMaterial _returnvalue))
  (Rendering|Material|SetMaterial (Variables|Default|Getmesh) 0 _output_get))