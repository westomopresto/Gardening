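; Ocean actor that refills the water supply held in GardenGameMode while the player is in it.
; Static mesh overlaps with mizu_character set an in-water flag, and Tick then adds water in fixed steps, using smaller increments near the maximum.
; Each gain plays a pickup sound, while a resettable DoOnce keeps the capacity sound from repeating when water is full.
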(event OnComponentBeginOverlap(StaticMeshComponent)
  (params (OverlappedComponent :type Primitive%20Component%20Object%20Reference) (OtherActor :type Actor%20Object%20Reference) (OtherComp :type Primitive%20Component%20Object%20Reference) (OtherBodyIndex :type Integer) (bFromSweep :type Boolean) (SweepResult :type Hit%20Result%20Structure%20%28by%20ref%29))
  (Utilities|Casting|CastTomizu_character OtherActor)
  (Variables|Default|SetplayerInWater true))

(event OnComponentEndOverlap(StaticMeshComponent)
  (params (OverlappedComponent :type Primitive%20Component%20Object%20Reference) (OtherActor :type Actor%20Object%20Reference) (OtherComp :type Primitive%20Component%20Object%20Reference) (OtherBodyIndex :type Integer))
  (Utilities|Casting|CastTomizu_character OtherActor)
  (Variables|Default|SetplayerInWater false)
  (CallFunction|ResetCapacitySFX))

(event Custom|resetCapacitySFX
  (Utilities|FlowControl|DoOnce false) ; enters at Reset
)

(event Custom|playCapacitySFX
  (Utilities|FlowControl|DoOnce false
    (:Completed
      (Audio|PlaySound2D "/Game/sounds/water_capacity.water_capacity" 1.0 1.0 0.0 0 0))))

(event EventBeginPlay)

(event Collision|EventActorBeginOverlap
  (params (OtherActor :type Actor%20Object%20Reference)))

(event EventTick
  (params (DeltaSeconds :type Float%20%28single-precision%29))
  (if (Variables|Default|GetplayerInWater)
    (bind _asgarden_game_mode (Utilities|Casting|CastToGardenGameMode (Game|GetGameMode)))
    (if (< (Variables|/Game/Blueprints/Blueprints/GardenGameMode.GardenGameMode_C|Getwater _asgarden_game_mode) (Variables|/Game/Blueprints/Blueprints/GardenGameMode.GardenGameMode_C|GetmaxWater _asgarden_game_mode))
      (if (> (+ (Variables|/Game/Blueprints/Blueprints/GardenGameMode.GardenGameMode_C|Getwater _asgarden_game_mode) 10) (Variables|/Game/Blueprints/Blueprints/GardenGameMode.GardenGameMode_C|GetmaxWater _asgarden_game_mode))
        (if (< (+ (Variables|/Game/Blueprints/Blueprints/GardenGameMode.GardenGameMode_C|Getwater _asgarden_game_mode) (- (+ (Variables|/Game/Blueprints/Blueprints/GardenGameMode.GardenGameMode_C|Getwater _asgarden_game_mode) 10) (Variables|/Game/Blueprints/Blueprints/GardenGameMode.GardenGameMode_C|GetmaxWater _asgarden_game_mode))) (Variables|/Game/Blueprints/Blueprints/GardenGameMode.GardenGameMode_C|GetmaxWater _asgarden_game_mode))
          (Variables|/Game/Blueprints/Blueprints/GardenGameMode.GardenGameMode_C|Setwater _asgarden_game_mode (+ (Variables|/Game/Blueprints/Blueprints/GardenGameMode.GardenGameMode_C|Getwater _asgarden_game_mode) (- (+ (Variables|/Game/Blueprints/Blueprints/GardenGameMode.GardenGameMode_C|Getwater _asgarden_game_mode) 10) (Variables|/Game/Blueprints/Blueprints/GardenGameMode.GardenGameMode_C|GetmaxWater _asgarden_game_mode))))
          (else
            (Variables|/Game/Blueprints/Blueprints/GardenGameMode.GardenGameMode_C|Setwater _asgarden_game_mode (+ (Variables|/Game/Blueprints/Blueprints/GardenGameMode.GardenGameMode_C|Getwater _asgarden_game_mode) 1))))
        (else
          (Variables|/Game/Blueprints/Blueprints/GardenGameMode.GardenGameMode_C|Setwater _asgarden_game_mode (+ (Variables|/Game/Blueprints/Blueprints/GardenGameMode.GardenGameMode_C|Getwater _asgarden_game_mode) 10))))
      (Audio|PlaySound2D "/Game/sounds/water_pickup.water_pickup" 1.0 1.0 0.0 0 0)
      (CallFunction|ResetCapacitySFX)
      (if (>= (Variables|/Game/Blueprints/Blueprints/GardenGameMode.GardenGameMode_C|Getwater _asgarden_game_mode) (Variables|/Game/Blueprints/Blueprints/GardenGameMode.GardenGameMode_C|GetmaxWater _asgarden_game_mode))
        (CallFunction|PlayCapacitySFX))
      (else
        (Utilities|FlowControl|DoOnce false
          (:Completed
            (Audio|PlaySound2D "/Game/sounds/water_capacity.water_capacity" 1.0 1.0 0.0 0 0)))))))

(fn ConstructionScript)