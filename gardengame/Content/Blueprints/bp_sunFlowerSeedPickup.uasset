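; Seed pickup actor that adds a Sunflower or Cactus seed to the garden game's inventory when the player walks into it.
; On box overlap by mizu_character, it switches on SeedType to increment the matching seed count on GardenGameMode.
; Both branches then play a high-pitched harvest sound, bump the seeds-found stat and destroy the pickup.
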(event OnComponentBeginOverlap(Box)
  (params (OverlappedComponent :type Primitive%20Component%20Object%20Reference) (OtherActor :type Actor%20Object%20Reference) (OtherComp :type Primitive%20Component%20Object%20Reference) (OtherBodyIndex :type Integer) (bFromSweep :type Boolean) (SweepResult :type Hit%20Result%20Structure%20%28by%20ref%29))
  (Utilities|Casting|CastTomizu_character OtherActor)
  (bind _asgarden_game_mode (Utilities|Casting|CastToGardenGameMode (Game|GetGameMode)))
  (switch Utilities|FlowControl|Switch|SwitchonseedTypes (Variables|Default|GetseedType)
    (:NewEnumerator1
      (Variables|/Game/Blueprints/Blueprints/GardenGameMode.GardenGameMode_C|SetFLOWER_seeds _asgarden_game_mode (+ (Variables|/Game/Blueprints/Blueprints/GardenGameMode.GardenGameMode_C|GetFLOWER_seeds _asgarden_game_mode) 1)))
    (:NewEnumerator2
      (Variables|/Game/Blueprints/Blueprints/GardenGameMode.GardenGameMode_C|SetCACTUS_seeds _asgarden_game_mode (+ (Variables|/Game/Blueprints/Blueprints/GardenGameMode.GardenGameMode_C|GetCACTUS_seeds _asgarden_game_mode) 1))))
  (Audio|PlaySound2D "/Game/sounds/harvest.harvest" 1.0 2.0 0.0 0 0)
  (Variables|/Game/Blueprints/Blueprints/GardenGameMode.GardenGameMode_C|SetgameStat_SEEDS_FOUND _asgarden_game_mode (+ (Variables|/Game/Blueprints/Blueprints/GardenGameMode.GardenGameMode_C|GetgameStat_SEEDS_FOUND _asgarden_game_mode) 1))
  (Actor|DestroyActor))

(event EventBeginPlay)

(event Collision|EventActorBeginOverlap
  (params (OtherActor :type Actor%20Object%20Reference)))

(event EventTick
  (params (DeltaSeconds :type Float%20%28single-precision%29)))

(fn ConstructionScript)