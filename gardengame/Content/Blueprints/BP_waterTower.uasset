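; BP_waterTower is a water tower actor in a garden game, with a Water component that uses its own material.
; The construction script creates a dynamic instance of M_WaterTower, stores it and applies it to the Water component.
; Tick only casts the game mode to GardenGameMode.
; Nodes for scaling height from the game mode's Water value are left unconnected, so the level never updates here.
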(event EventBeginPlay)

(event Collision|EventActorBeginOverlap
  (params (OtherActor :type Actor%20Object%20Reference)))

(event EventTick
  (params (DeltaSeconds :type Float%20%28single-precision%29))
  (bind _asgarden_game_mode (Utilities|Casting|CastToGardenGameMode (Game|GetGameMode))))

(fn ConstructionScript
  (bind _returnvalue (Rendering|Material|CreateDynamicMaterialInstance "/Game/Shaders/M_WaterTower.M_WaterTower" "None" :!class /Script/Engine.KismetMaterialLibrary))
  (bind _output_get (Variables|Default|SetdynamicMaterial _returnvalue))
  (Rendering|Material|SetMaterial (Variables|Default|Getwater) 0 _output_get))