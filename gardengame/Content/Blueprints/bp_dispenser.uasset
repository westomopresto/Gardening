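; A clickable garden dispenser that trades the game mode's Energy for either seeds or a one-time watering can upgrade, as set by PurchaseSeed.
; Seed purchases add Sunflower or Cactus seeds to the game mode, while the upgrade flags the player character and disables the dispenser.
; Sounds and a timeline-driven emissive color on a dynamic material give feedback.
; The construction script sets the displayed meshes and price text.
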(event Custom|purchaseSeeds
  (CallFunction|SuccessColor)
  (bind _asgarden_game_mode (Utilities|Casting|CastToGardenGameMode (Game|GetGameMode)))
  (switch Utilities|FlowControl|Switch|SwitchonseedTypes (Variables|Default|GetseedToSell)
    (:NewEnumerator1
      (Variables|/Game/Blueprints/Blueprints/GardenGameMode.GardenGameMode_C|SetFLOWER_seeds _asgarden_game_mode (+ (Variables|/Game/Blueprints/Blueprints/GardenGameMode.GardenGameMode_C|GetFLOWER_seeds _asgarden_game_mode) (Variables|Default|GetamountGiven))))
    (:NewEnumerator2
      (Variables|/Game/Blueprints/Blueprints/GardenGameMode.GardenGameMode_C|SetCACTUS_seeds _asgarden_game_mode (+ (Variables|/Game/Blueprints/Blueprints/GardenGameMode.GardenGameMode_C|GetCACTUS_seeds _asgarden_game_mode) (Variables|Default|GetamountGiven))))))

(event Custom|purchaseUpgrade
  (Variables|Default|Setdisable true)
  (Rendering|Material|SetVectorParameterValue (Variables|Default|Getdynamic_Material) "eColor" "(R=0.000000,G=0.000000,B=0.000000,A=1.000000)" :!class /Script/Engine.MaterialInstanceDynamic)
  (bind _asmizu_character (Utilities|Casting|CastTomizu_character (Game|Player|GetPlayerPawn 0)))
  (Variables|/Game/Blueprints/Blueprints/mizu_character.mizu_character_C|SetwaterCanUpgrade _asmizu_character true)
  (Default|PropSelection _asmizu_character))

(event Custom|successColor
  (bind _dynamic_material (Variables|Default|Getdynamic_Material))
  (Audio|PlaySound2D "/Game/sounds/purchase.purchase" 1.0 1.0 0.0 0 0)
  (Rendering|Material|SetVectorParameterValue _dynamic_material "eColor" "(R=0.000000,G=1.000000,B=0.184041,A=1.000000)" :!class /Script/Engine.MaterialInstanceDynamic)
  (bind _alpha (Timeline|Timeline_0 PlayFromStart)
    (:Update
      (Rendering|Material|SetScalarParameterValue _dynamic_material "emission" _alpha :!class /Script/Engine.MaterialInstanceDynamic))))

(event Custom|failColor
  (bind _dynamic_material (Variables|Default|Getdynamic_Material))
  (Audio|PlaySound2D "/Game/sounds/deny.deny" 2.0 1.0 0.0 0 0)
  (Rendering|Material|SetVectorParameterValue _dynamic_material "eColor" "(R=1.000000,G=0.154483,B=0.078125,A=1.000000)" :!class /Script/Engine.MaterialInstanceDynamic)
  (bind _alpha (Timeline|Timeline_0 PlayFromStart)
    (:Update
      (Rendering|Material|SetScalarParameterValue _dynamic_material "emission" _alpha :!class /Script/Engine.MaterialInstanceDynamic))))

(event Custom|waitColor
  (bind _dynamic_material (Variables|Default|Getdynamic_Material))
  (Audio|PlaySound2D "/Game/sounds/deny.deny" 1.0 1.0 0.0 0 0)
  (Rendering|Material|SetVectorParameterValue _dynamic_material "eColor" "(R=1.000000,G=0.968331,B=0.000000,A=1.000000)" :!class /Script/Engine.MaterialInstanceDynamic)
  (bind _alpha (Timeline|Timeline_0 PlayFromStart)
    (:Update
      (Rendering|Material|SetScalarParameterValue _dynamic_material "emission" _alpha :!class /Script/Engine.MaterialInstanceDynamic))))

(event EventBeginPlay)

(event Collision|EventActorBeginOverlap
  (params (OtherActor :type Actor%20Object%20Reference)))

(event EventTick
  (params (DeltaSeconds :type Float%20%28single-precision%29)))

(event MouseInput|EventActorOnClicked
  (params (ButtonPressed :type Key%20Structure))
  (if (Variables|Default|Getdisable)
    (CallFunction|FailColor)
    (else
      (bind _asgarden_game_mode (Utilities|Casting|CastToGardenGameMode (Game|GetGameMode)))
      (if (>= (Variables|/Game/Blueprints/Blueprints/GardenGameMode.GardenGameMode_C|Getenergy _asgarden_game_mode) (Variables|Default|Getcost))
        (Variables|/Game/Blueprints/Blueprints/GardenGameMode.GardenGameMode_C|Setenergy _asgarden_game_mode (- (Variables|/Game/Blueprints/Blueprints/GardenGameMode.GardenGameMode_C|Getenergy _asgarden_game_mode) (Variables|Default|Getcost)))
        (if (Variables|Default|GetpurchaseSeed?)
          (CallFunction|PurchaseSeeds)
          (else
            (CallFunction|PurchaseUpgrade)))
        (else
          (CallFunction|FailColor))))))

(fn ConstructionScript
  (bind _staticmesh (Variables|Default|GetStaticMesh))
  (bind _skeletalmesh (Variables|Default|GetSkeletalMesh))
  (Utilities|FlowControl|Sequence
    (:then_0
      (if (Variables|Default|GetpurchaseSeed?)
        (switch Utilities|FlowControl|Switch|SwitchonseedTypes (Variables|Default|GetseedToSell)
          (:NewEnumerator0
            (Components|StaticMesh|SetStaticMesh _staticmesh "/Game/Geometry/Meshes/seed_01.seed_01" :!label _label)
            (Class|SkinnedMeshComponent|SetSkeletalMesh _skeletalmesh "/Game/Geometry/Meshes/sunFlower_0.sunFlower_0" true))
          (:NewEnumerator1
            (goto _label))
          (:NewEnumerator2
            (Components|StaticMesh|SetStaticMesh _staticmesh "/Game/Geometry/Meshes/cactus_seed_01.cactus_seed_01")
            (Class|SkinnedMeshComponent|SetSkeletalMesh _skeletalmesh "/Game/Geometry/Meshes/cactus_01.cactus_01" true))
          (:NewEnumerator3
            (goto _label)))
        (else
          (Rendering|SetVisibility (Variables|Default|GetStaticMesh) false false)
          (Rendering|SetVisibility (Variables|Default|GetSkeletalMesh) false false)
          (Rendering|SetVisibility (Variables|Default|Getitem) true false))))
    (:then_1
      (bind _returnvalue (Rendering|Material|CreateDynamicMaterialInstance "/Game/Shaders/circuit.circuit" "None" :!class /Script/Engine.KismetMaterialLibrary))
      (bind _output_get (Variables|Default|Setdynamic_Material _returnvalue))
      (Rendering|Material|SetMaterial (Variables|Debug|GetStaticMeshComponent) 0 _output_get))
    (:then_2
      (Rendering|Components|TextRender|SetText (Variables|Default|GetTextRender) (Utilities|Text|ToText(String) (Utilities|String|Append (Utilities|String|BuildString(Integer) "" "" (Variables|Default|Getcost) " energy") (Utilities|String|BuildString(Integer) " for " "" (Variables|Default|GetamountGiven))))))))