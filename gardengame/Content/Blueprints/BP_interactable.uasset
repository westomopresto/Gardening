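; Clickable energy receptacle actor that takes the player's energy and triggers a linked BP_door once full.
; A click within range moves one unit from GardenGameMode's Energy into CurrentEnergy; distant or invalid clicks play a deny sound.
; A dynamic material flashes green, red or yellow through a shared emission timeline.
; Tick refreshes the remaining-energy text and bar scale, firing completion once through DoOnce.
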(event Custom|interact
  (bind _asgarden_game_mode (Utilities|Casting|CastToGardenGameMode (Game|GetGameMode)))
  (if (and (> (Variables|/Game/Blueprints/Blueprints/GardenGameMode.GardenGameMode_C|Getenergy _asgarden_game_mode) 0) (not (== (Variables|Default|GetcurrentEnergy) (Variables|Default|GetrequiredEnergy))))
    (Variables|/Game/Blueprints/Blueprints/GardenGameMode.GardenGameMode_C|Setenergy _asgarden_game_mode (- (Variables|/Game/Blueprints/Blueprints/GardenGameMode.GardenGameMode_C|Getenergy _asgarden_game_mode) 1))
    (Variables|Default|SetcurrentEnergy (+ (Variables|Default|GetcurrentEnergy) 1))
    (CallFunction|SuccessColor)
    (Audio|PlaySound2D "/Game/sounds/energyDeposit.energyDeposit" 3.0 2.0 0.0 0 0)
    (else
      (CallFunction|FailColor))))

(event Custom|complete
  (bind _doortoopen (Variables|Default|GetdoorToOpen))
  (Utilities|IsValid _doortoopen
    (:Is%20Valid
      (bind _asb_p_door (Utilities|Casting|CastTobP_door _doortoopen))
      (Default|Casted _asb_p_door))))

(event Custom|playActionAnim
  (bind _asmizu_character (Utilities|Casting|CastTomizu_character (Game|Player|GetPlayerPawn 0)))
  (Default|PlayActionMontage _asmizu_character false))

(event Custom|forceUpdate
  (bind _requiredenergy (Variables|Default|GetrequiredEnergy))
  (bind _textrender (Variables|Default|GetTextRender))
  (bind _currentenergy (Variables|Default|GetcurrentEnergy))
  (bind _returnvalue (- _requiredenergy _currentenergy))
  (if (== _returnvalue 0)
    (Rendering|Components|TextRender|SetText _textrender (Utilities|Text|MakeLiteralText "ENERGY<br>FULL"))
    (Transformation|SetRelativeScale3D (Variables|Default|GetenergyScale) (Math|Vector|MakeVector 1.0 1.0 1.0))
    (Utilities|FlowControl|DoOnce false
      (:Completed
        (CallFunction|Complete)))
    (else
      (Rendering|Components|TextRender|SetText _textrender (Utilities|Text|ToText(String) (Utilities|String|BuildString(Integer) "ENERGY <br>NEEDED: " "" _returnvalue)))
      (Transformation|SetRelativeScale3D (Variables|Default|GetenergyScale) (Math|Vector|MakeVector 1.0 1.0 (Math|Float|Lerp 0.25 1.0 (/ (Math|Conversions|ToFloat(Integer) _currentenergy) (Math|Conversions|ToFloat(Integer) _requiredenergy))))))))

(event Custom|successColor
  (bind _dynamic_material (Variables|Default|Getdynamic_Material))
  (Rendering|Material|SetVectorParameterValue _dynamic_material "eColor" "(R=0.000000,G=1.000000,B=0.184041,A=1.000000)" :!class /Script/Engine.MaterialInstanceDynamic)
  (bind _alpha (Timeline|Timeline_0 PlayFromStart)
    (:Update
      (Rendering|Material|SetScalarParameterValue _dynamic_material "emission" _alpha :!class /Script/Engine.MaterialInstanceDynamic))))

(event Custom|failColor
  (bind _dynamic_material (Variables|Default|Getdynamic_Material))
  (Audio|PlaySound2D "/Game/sounds/deny.deny" 2.0 1.0 0.0 0 0)
  (Rendering|Material|SetVectorParameterValue _dynamic_material "eColor" "(R=1.000000,G=0.154483,B=0.078125,A=1.000000)" :!class /Script/Engine.MaterialInstanceDynamic)
  (bind _alpha (Timeline|Timeline_0 PlayFromStart)
    (:Update
      (Rendering|Material|SetScalarParameterValue _dynamic_material "emission" _alpha :!class /Script/Engine.MaterialInstanceDynamic))))

(event Custom|waitColor
  (bind _dynamic_material (Variables|Default|Getdynamic_Material))
  (Audio|PlaySound2D "/Game/sounds/deny.deny" 1.0 1.0 0.0 0 0)
  (Rendering|Material|SetVectorParameterValue _dynamic_material "eColor" "(R=1.000000,G=0.968331,B=0.000000,A=1.000000)" :!class /Script/Engine.MaterialInstanceDynamic)
  (bind _alpha (Timeline|Timeline_0 PlayFromStart)
    (:Update
      (Rendering|Material|SetScalarParameterValue _dynamic_material "emission" _alpha :!class /Script/Engine.MaterialInstanceDynamic))))

(event EventBeginPlay)

(event Collision|EventActorBeginOverlap
  (params (OtherActor :type Actor%20Object%20Reference)))

(event EventTick
  (params (DeltaSeconds :type Float%20%28single-precision%29))
  (bind _requiredenergy (Variables|Default|GetrequiredEnergy))
  (bind _textrender (Variables|Default|GetTextRender))
  (bind _currentenergy (Variables|Default|GetcurrentEnergy))
  (bind _returnvalue (- _requiredenergy _currentenergy))
  (if (== _returnvalue 0)
    (Rendering|Components|TextRender|SetText _textrender (Utilities|Text|MakeLiteralText "ENERGY<br>FULL"))
    (Transformation|SetRelativeScale3D (Variables|Default|GetenergyScale) (Math|Vector|MakeVector 1.0 1.0 1.0))
    (Utilities|FlowControl|DoOnce false
      (:Completed
        (CallFunction|Complete)))
    (else
      (Rendering|Components|TextRender|SetText _textrender (Utilities|Text|ToText(String) (Utilities|String|BuildString(Integer) "ENERGY <br>NEEDED: " "" _returnvalue)))
      (Transformation|SetRelativeScale3D (Variables|Default|GetenergyScale) (Math|Vector|MakeVector 1.0 1.0 (Math|Float|Lerp 0.25 1.0 (/ (Math|Conversions|ToFloat(Integer) _currentenergy) (Math|Conversions|ToFloat(Integer) _requiredenergy))))))))

(event MouseInput|EventActorOnClicked
  (params (ButtonPressed :type Key%20Structure))
  (if (<= (Transformation|GetDistanceTo (Game|Player|GetPlayerPawn 0)) 2.4e+02)
    (CallFunction|Interact)
    (else
      (CallFunction|WaitColor))))

(fn ConstructionScript
  (bind _returnvalue (Rendering|Material|CreateDynamicMaterialInstance "/Game/Shaders/circuit.circuit" "None" :!class /Script/Engine.KismetMaterialLibrary))
  (bind _output_get (Variables|Default|Setdynamic_Material _returnvalue))
  (Rendering|Material|SetMaterial (Variables|Debug|GetStaticMeshComponent) 2 _output_get))