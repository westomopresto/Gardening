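; BP_soil is a soil actor whose material reflects its water level.
; The construction script creates a dynamic instance of M_soil_Grow, applies it to the static mesh and sets its "water" parameter from SoilWater divided by 100.
; Tick pushes the same value to the material every frame and prints SoilWater to the screen.
; Nothing in these graphs changes SoilWater itself.
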(event EventBeginPlay)

(event Collision|EventActorBeginOverlap
  (params (OtherActor :type Actor%20Object%20Reference)))

(event EventTick
  (params (DeltaSeconds :type Float%20%28single-precision%29))
  (bind _soil_water (Variables|Default|Getsoil_water))
  (Rendering|Material|SetScalarParameterValue (Variables|Default|Getsoil_material) "water" (/ (Math|Conversions|ToFloat(Integer) _soil_water) 1e+02) :!class /Script/Engine.MaterialInstanceDynamic)
  (Development|PrintString (Utilities|String|ToString(Integer) _soil_water)))

(fn ConstructionScript
  (bind _returnvalue (Rendering|Material|CreateDynamicMaterialInstance "/Game/Shaders/M_soil_Grow.M_soil_Grow" "None" :!class /Script/Engine.KismetMaterialLibrary))
  (bind _output_get (Variables|Default|Setsoil_material _returnvalue))
  (Rendering|Material|SetMaterial (Variables|Debug|GetStaticMeshComponent) 0 _output_get)
  (Rendering|Material|SetScalarParameterValue (Variables|Default|Getsoil_material) "water" (/ (Math|Conversions|ToFloat(Integer) (Variables|Default|Getsoil_water)) 1e+02) :!class /Script/Engine.MaterialInstanceDynamic))